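; Player character Blueprint that handles input for the inventory, the notepad and a noise-making action.
; Tab and N each drive their own FlipFlop, creating a fresh widget with the cursor shown and game paused, then removing it and reversing both.
; F emits a noise event at the character's location, plus a particle effect and a sound that use what look like placeholder assets.
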(event Collision|EventActorBeginOverlap
  (params (OtherActor :type Actor%20Object%20Reference)))

(event EventTick
  (params (DeltaSeconds :type Float%20%28single-precision%29)))

(event Input|KeyboardEvents|N
  (params (Key :type Key%20Structure :default "None"))
  (:Pressed
    (Utilities|FlowControl|FlipFlop
      (:A
        (bind _returnvalue (UserInterface|CreateWidget "/Game/Blueprints/Equipment/Widget/WBP_Notepad.WBP_Notepad_C"))
        (bind _output_get (Variables|Default|SetNotepad%20Ref _returnvalue))
        (UserInterface|Viewport|AddtoViewport _output_get 0)
        (Variables|/Script/Engine.PlayerController|SetbShowMouseCursor (Game|GetPlayerController 0) true)
        (Game|SetGamePaused true))
      (:B
        (Widget|RemovefromParent (Variables|Default|GetNotepad%20Ref))
        (Variables|/Script/Engine.PlayerController|SetbShowMouseCursor (Game|GetPlayerController 0) false)
        (Game|SetGamePaused false)))))

(event Input|KeyboardEvents|Tab
  (params (Key :type Key%20Structure :default "None"))
  (:Pressed
    (Utilities|FlowControl|FlipFlop
      (:A
        (bind _returnvalue (UserInterface|CreateWidget "/Game/Blueprints/Inventory/UI/WBP_InventoryUI.WBP_InventoryUI_C"))
        (bind _output_get (Variables|Default|SetInventory%20Ref _returnvalue))
        (UserInterface|Viewport|AddtoViewport _output_get 0)
        (Variables|/Script/Engine.PlayerController|SetbShowMouseCursor (Game|GetPlayerController 0) true)
        (Game|SetGamePaused true))
      (:B
        (Widget|RemovefromParent (Variables|Default|GetInventory%20Ref))
        (Variables|/Script/Engine.PlayerController|SetbShowMouseCursor (Game|GetPlayerController 0) false)
        (Game|SetGamePaused false)))))

(event Input|KeyboardEvents|F
  (params (Key :type Key%20Structure :default "None"))
  (bind _returnvalue (Transformation|GetActorLocation))
  (:Pressed
    (Class|Actor|MakeNoise 1.0 self _returnvalue 0.0 "None")
    (Effects|SpawnEmitteratLocation "/Engine/Tutorial/SubEditors/TutorialAssets/TutorialParticleSystem.TutorialParticleSystem" "0, 0, 0")
    (Audio|PlaySoundatLocation "/Engine/EditorSounds/Notifications/CompileSuccess.CompileSuccess" _returnvalue "0, 0, 0" 1.0 1.0 0.0 0 0 0 0)))

(fn ConstructionScript)